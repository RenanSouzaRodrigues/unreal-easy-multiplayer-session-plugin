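; BP_PlayerCharacter is the player-controlled character, handling movement, camera, jumping, sprinting and weapon use.
; On BeginPlay it creates WBP_PlayerWidget and adds it to the viewport.
; Enhanced Input actions forward to separate functions for moving, looking, jumping, sprinting, equipping, aiming and firing.
; Sprint and aim are hold actions that stop on either Completed or Canceled, while equip fires on Completed.
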(event `self.ReceiveBeginPlay`
  (bind _returnvalue (`|CreateWidget` "/Game/GameAssets/Blueprints/Widgets/WBP_PlayerWidget.WBP_PlayerWidget_C"))
  (`UserWidget.AddToViewport` _returnvalue 0))

(event `EnhancedInput|/Game/GameAssets/Blueprints/Inputs/IA_Movement`
  (params (ActionValue :type "Vector2D Structure") (ElapsedSeconds :type "Float (double-precision)") (TriggeredSeconds :type "Float (double-precision)") (InputAction :type "InputAction Object Reference" :default "/Game/GameAssets/Blueprints/Inputs/IA_Movement.IA_Movement"))
  (:`Triggered`
    (`self.MovePlayer` ActionValue_X ActionValue_Y)))

(event `EnhancedInput|/Game/GameAssets/Blueprints/Inputs/IA_MoveCamera`
  (params (ActionValue :type "Vector2D Structure") (ElapsedSeconds :type "Float (double-precision)") (TriggeredSeconds :type "Float (double-precision)") (InputAction :type "InputAction Object Reference" :default "/Game/GameAssets/Blueprints/Inputs/IA_MoveCamera.IA_MoveCamera"))
  (:`Triggered`
    (`self.MoveCamera` ActionValue_X ActionValue_Y)))

(event `EnhancedInput|/Game/GameAssets/Blueprints/Inputs/IA_Jump`
  (params (ActionValue :type Boolean) (ElapsedSeconds :type "Float (double-precision)") (TriggeredSeconds :type "Float (double-precision)") (InputAction :type "InputAction Object Reference" :default "/Game/GameAssets/Blueprints/Inputs/IA_Jump.IA_Jump"))
  (:`Started`
    (`self.PerformJump`)))

(event `EnhancedInput|/Game/GameAssets/Blueprints/Inputs/IA_Sprint`
  (params (ActionValue :type Boolean) (ElapsedSeconds :type "Float (double-precision)") (TriggeredSeconds :type "Float (double-precision)") (InputAction :type "InputAction Object Reference" :default "/Game/GameAssets/Blueprints/Inputs/IA_Sprint.IA_Sprint"))
  (:`Started`
    (`self.Sprint`))
  (:`Canceled`
    (`self.StopSprint` :!label _label))
  (:`Completed`
    (goto _label)))

(event `EnhancedInput|/Game/GameAssets/Blueprints/Inputs/IA_EquipWeapon`
  (params (ActionValue :type Boolean) (ElapsedSeconds :type "Float (double-precision)") (TriggeredSeconds :type "Float (double-precision)") (InputAction :type "InputAction Object Reference" :default "/Game/GameAssets/Blueprints/Inputs/IA_EquipWeapon.IA_EquipWeapon"))
  (:`Completed`
    (`self.EquipWeapon`)))

(event `EnhancedInput|/Game/GameAssets/Blueprints/Inputs/IA_Aim`
  (params (ActionValue :type Boolean) (ElapsedSeconds :type "Float (double-precision)") (TriggeredSeconds :type "Float (double-precision)") (InputAction :type "InputAction Object Reference" :default "/Game/GameAssets/Blueprints/Inputs/IA_Aim.IA_Aim"))
  (:`Started`
    (`self.AimWeapon`))
  (:`Canceled`
    (`self.StopAimWeapon` :!label _label_2))
  (:`Completed`
    (goto _label_2)))

(event `EnhancedInput|/Game/GameAssets/Blueprints/Inputs/IA_Shoot`
  (params (ActionValue :type Boolean) (ElapsedSeconds :type "Float (double-precision)") (TriggeredSeconds :type "Float (double-precision)") (InputAction :type "InputAction Object Reference" :default "/Game/GameAssets/Blueprints/Inputs/IA_Shoot.IA_Shoot"))
  (:`Started`
    (`self.FireWeapon`)))

(fn `UserConstructionScript`)